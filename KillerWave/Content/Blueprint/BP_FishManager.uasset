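; BP_FishManager is a Blueprint that counts fish and detects when the win total is reached.
; BeginPlay resets the count to zero, and the AddFish event increments it and prints the new value.
; Once the count reaches or exceeds TotalFishToWin, it only prints a "Win" message, with no other win logic.
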(event `AddFish`
  (bind _output_get (set `self.FishCount` (+ (`self.FishCount`) 1)))
  (`KismetSystemLibrary.PrintString` (`KismetStringLibrary.Conv_IntToString` _output_get))
  (if (>= _output_get (`self.TotalFishToWin`))
    (`KismetSystemLibrary.PrintString` "Win")))

(event `self.ReceiveBeginPlay`
  (set `self.FishCount` 0))

(fn `UserConstructionScript`)