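; BP_JellyFish is a jellyfish that flees from fish and static meshes entering its Sphere trigger.
; Each tick it pitches its skeletal mesh in proportion to the inherited CurrentSpeed.
; On overlap with a FishCharacter it calls Escape from that fish's location, and a BP_KillerFish is also made to escape from the jellyfish.
; For static mesh overlaps it escapes from a point just ahead of itself.
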(event `self.ReceiveTick`
  (params (DeltaSeconds :type "Float (single-precision)"))
  (`parent.ReceiveTick` DeltaSeconds)
  (`SceneComponent.K2_SetRelativeRotation` (`self.SkeletalMesh`) (`KismetMathLibrary.MakeRotator` 0.0 (/ (`self.CurrentSpeed`) -3.5)) false false))

(event `self.Sphere.OnComponentBeginOverlap`
  (params (OverlappedComponent :type "PrimitiveComponent Object Reference") (OtherActor :type "Actor Object Reference") (OtherComp :type "PrimitiveComponent Object Reference") (OtherBodyIndex :type Integer) (bFromSweep :type Boolean) (SweepResult :type "HitResult Structure (by ref)"))
  (bind _asfish_character (cast `FishCharacter` OtherActor)
    (:`then`
      (`self.Escape` (`self.K2_GetActorLocation` _asfish_character))
      (bind _asbp_killer_fish (cast `/Game/Blueprint/BP_KillerFish` OtherActor))
      (`self.Escape` _asbp_killer_fish (`self.K2_GetActorLocation`)))
    (:`CastFailed`
      (cast `StaticMeshComponent` OtherComp)
      (`self.Escape` (+ (* (`self.GetActorForwardVector`) 100.0) (`self.K2_GetActorLocation`))))))

(fn `UserConstructionScript`
  (`parent.UserConstructionScript`))